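; Checkpoint is a race checkpoint actor with a trigger volume and two side markers that reports when players pass through it.
; When a pawn overlaps it, it sends the player ID, game time and its StartFinish value to the RaceMode game mode.
; The construction script scales the trigger and spaces the left and right pollers from a Width variable, so the gate resizes in the editor.
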(event EventActorBeginOverlap
  (params (OtherActor :type Actor%20Object%20Reference))
  (bind _aspawn (Utilities|Casting|CastToPawn OtherActor))
  (bind _asrace_mode (Utilities|Casting|CastToRaceMode (Game|GetGameMode)))
  (Class|RaceMode|RegisterCheckpointTime _asrace_mode (Variables|/Script/Engine.PlayerState|GetPlayerId (Variables|/Script/Engine.Pawn|GetPlayerState _aspawn)) (Utilities|Time|GetGameTimeinSeconds) (Variables|Default|GetStartFinish)))

(fn ConstructionScript
  (Transformation|SetRelativeScale3D (Variables|Default|GetTrigger) (Math|Vector|MakeVector 1.0 (Variables|Default|GetWidth) 2e+01))
  (Transformation|SetRelativeLocation (Variables|Default|GetLeftPoller) (Math|Vector|MakeVector 0.0 (* (Variables|Default|GetWidth) (/ 8.4e+02 25.0)) -6.5e+02) false)
  (Transformation|SetRelativeLocation (Variables|Default|GetRightPoller) (Math|Vector|MakeVector 0.0 (* (Variables|Default|GetWidth) (/ -8.4e+02 25.0)) -6.5e+02) false))